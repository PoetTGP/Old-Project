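; Moving actor for a platformer kit that slides its mesh pivot through a list of relative Destinations, starting on BeginPlay or on SimpleActivate.
; The construction script applies size and material and snaps the pivot to the starting destination.
; A timeline lerps each leg, with play rate set from Speed over distance, then waits WaitTime before the next.
; With Looping it wraps to the first point; DoOnce blocks repeat activation.
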(event `self.ReceiveBeginPlay`
  (bind _destinations (`self.Destinations`))
  (bind _returnvalue (+ (`self.Index`) 1))
  (bind _returnvalue_2 (select `bool` (`KismetArrayLibrary.Array_IsValidIndex` _destinations _returnvalue) :`true` _returnvalue))
  (if (`self.BeginAutomatically`)
    (if (>= (`KismetArrayLibrary.Array_Length` (`self.Destinations`)) 2) :!label _label
      (`/Engine/EditorBlueprintResources/StandardMacros.DoOnce` false
        (:`Completed`
          (set `self.End` (`|GetArrayItem` _destinations _returnvalue_2) :!label _label_2)
          (set `self.Index` _returnvalue_2)
          (`TimelineComponent.SetPlayRate` (`self.Movement`) (/ (`self.Speed`) (`KismetMathLibrary.Vector_Distance` (`self.Start`) (`self.End`))))
          (bind (_direction _alpha) (`Timeline|Movement` :!via `PlayFromStart`)
            (:`Update`
              (`SceneComponent.K2_SetRelativeLocation` (`self.Pivot`) (`KismetMathLibrary.VLerp` (`self.Start`) (`self.End`) _alpha) false false))
            (:`Finished`
              (if (`KismetArrayLibrary.Array_IsValidIndex` (`self.Destinations`) (+ (`self.Index`) 1))
                (set `self.Start` (`self.End`) :!label _label_3)
                (`KismetSystemLibrary.Delay` (`self.WaitTime`))
                (`self.Replay`)
                (elif (`self.Looping`)
                  (goto _label_3))))))))))

(event `Replay`
  (goto _label_2))

(event `/Game/SimplePlatformerKit/Blueprints/Data/SimpleBPI.SimpleActivate`
  (goto _label))

(fn `CheckKey`
  (params (KeyType :type "/Game/SimplePlatformerKit/Blueprints/Data/KeyType Enum" :default "NewEnumerator2"))
  (returns (Result :type Boolean))
  (return false))

(fn `UserConstructionScript`
  (`SceneComponent.SetRelativeScale3D` (`self.Pivot`) (`self.Size`))
  (`PrimitiveComponent.SetMaterial` (`self.Mesh`) 0 (`self.Material`))
  (bind _output_get (set `self.Start` (`|GetArrayItem` (`self.Destinations`) (`self.Index`))))
  (`SceneComponent.K2_SetRelativeLocation` (`self.Pivot`) _output_get false false))