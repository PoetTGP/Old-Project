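; Platformer door actor that opens for the player when they hold a key matching its KeyType color.
; On box overlap it sends a CheckKeyMessage to the Player-tagged actor and, on success, runs once.
; A Movement timeline then lerps the door mesh from its current relative location to End.
; The construction script sets the door's glow material to blue, yellow or purple based on KeyType.
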(event `self.Box.OnComponentBeginOverlap`
  (params (OverlappedComponent :type "PrimitiveComponent Object Reference") (OtherActor :type "Actor Object Reference") (OtherComp :type "PrimitiveComponent Object Reference") (OtherBodyIndex :type Integer) (bFromSweep :type Boolean) (SweepResult :type "HitResult Structure (by ref)"))
  (if (`self.ActorHasTag` OtherActor "Player")
    (bind _result (message `/Game/SimplePlatformerKit/Blueprints/Data/SimpleBPI.CheckKey` OtherActor (`self.KeyType`)))
    (if _result
      (`/Engine/EditorBlueprintResources/StandardMacros.DoOnce` false
        (:`Completed`
          (set `self.Start` (`SceneComponent.RelativeLocation` (`self.Door`)))
          (bind (_direction _alpha) (`Timeline|Movement`)
            (:`Update`
              (`SceneComponent.K2_SetRelativeLocation` (`self.Door`) (`KismetMathLibrary.VLerp` (`self.Start`) (`self.End`) _alpha) false false))))))))

(fn `UserConstructionScript`
  (`PrimitiveComponent.SetMaterial` (`self.Door`) 1 (select `/Game/SimplePlatformerKit/Blueprints/Data/KeyType` (`self.KeyType`) :`NewEnumerator2` "/Game/SimplePlatformerKit/Materials/SimpleMaterial/AssetMaterials/MI_BlueGlow.MI_BlueGlow" :`NewEnumerator1` "/Game/SimplePlatformerKit/Materials/SimpleMaterial/AssetMaterials/MI_YellowGlow.MI_YellowGlow" :`NewEnumerator0` "/Game/SimplePlatformerKit/Materials/SimpleMaterial/AssetMaterials/MI_PurpleGlow.MI_PurpleGlow" :!type "MaterialInterface Object Reference")))