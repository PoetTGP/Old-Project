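; Checkpoint actor from the simple platformer kit that registers itself as the player's checkpoint on capsule overlap.
; An overlapping actor tagged Player receives the checkpoint reference and a location offset from the capsule's world position through SetCheckpointMessage.
; A DoOnce gate shows the W_Checkpoint widget for a short time, then resets after a further delay, so repeat overlaps do not stack notifications.
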(event `self.Capsule.OnComponentBeginOverlap`
  (params (OverlappedComponent :type "PrimitiveComponent Object Reference") (OtherActor :type "Actor Object Reference") (OtherComp :type "PrimitiveComponent Object Reference") (OtherBodyIndex :type Integer) (bFromSweep :type Boolean) (SweepResult :type "HitResult Structure (by ref)"))
  (if (`self.ActorHasTag` OtherActor "Player")
    (message `/Game/SimplePlatformerKit/Blueprints/Data/SimpleBPI.SetCheckpoint` OtherActor self (+ (`self.CheckpointLocation`) (`SceneComponent.K2_GetComponentLocation` (`self.Capsule`))))
    (`/Engine/EditorBlueprintResources/StandardMacros.DoOnce` false :!label _label
      (:`Completed`
        (bind _returnvalue (`|CreateWidget` "/Game/SimplePlatformerKit/Blueprints/UI/W_Checkpoint.W_Checkpoint_C"))
        (`UserWidget.AddToViewport` _returnvalue 0)
        (`KismetSystemLibrary.Delay` 2.0)
        (`Widget.RemoveFromParent` _returnvalue)
        (`KismetSystemLibrary.Delay` 1.0)
        (`self.ResetDelay`)))))

(event `ResetDelay`
  (goto _label :!via `Reset`))

(fn `UserConstructionScript`)