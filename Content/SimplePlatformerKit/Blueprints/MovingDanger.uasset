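; MovingDanger is a platformer hazard that travels between destination points and sends any overlapping SimpleCharacter back to its respawn location.
; A timeline lerps the pivot along each leg at a distance-corrected speed, waiting between legs and optionally looping.
; Movement starts on BeginPlay or through SimpleActivate, gated by a DoOnce that an optional reset on overlap re-arms after returning the hazard to its first point.
; The construction script applies size, material and starting position.
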(event `self.ReceiveBeginPlay`
  (bind _returnvalue (+ (`self.Index`) 1))
  (if (`self.BeginAutomatically`)
    (if (>= (`KismetArrayLibrary.Array_Length` (`self.Destinations`)) 2) :!label _label
      (`/Engine/EditorBlueprintResources/StandardMacros.DoOnce` false :!label _label_2
        (:`Completed`
          (set `self.ForcedStop` false)
          (set `self.End` (`|GetArrayItem` (`self.Destinations`) 1))
          (`TimelineComponent.SetPlayRate` (`self.Movement`) (/ (`self.Speed`) (`KismetMathLibrary.Vector_Distance` (`self.Start`) (`self.End`))) :!label _label_3)
          (bind (_direction _alpha) (`Timeline|Movement` :!via `PlayFromStart`)
            (:`Update`
              (`SceneComponent.K2_SetRelativeLocation` (`self.Pivot`) (`KismetMathLibrary.VLerp` (`self.Start`) (`self.End`) _alpha) false false))
            (:`Finished`
              (if (`self.ForcedStop`)
                _
                (elif (`KismetArrayLibrary.Array_IsValidIndex` (`self.Destinations`) _returnvalue)
                  (set `self.Index` _returnvalue)
                  (set `self.Start` (`self.End`) :!label _label_4)
                  (set `self.End` (`|GetArrayItem` (`self.Destinations`) (`self.Index`)))
                  (`KismetSystemLibrary.Delay` (`self.WaitTime`))
                  (`self.Replay`)
                  (else
                    (set `self.Index` 0)
                    (if (`self.Looping`)
                      (goto _label_4))))))))))))

(event `Replay`
  (goto _label_3))

(event `/Game/SimplePlatformerKit/Blueprints/Data/SimpleBPI.SimpleActivate`
  (goto _label))

(event `self.Box.OnComponentBeginOverlap`
  (params (OverlappedComponent :type "PrimitiveComponent Object Reference") (OtherActor :type "Actor Object Reference") (OtherComp :type "PrimitiveComponent Object Reference") (OtherBodyIndex :type Integer) (bFromSweep :type Boolean) (SweepResult :type "HitResult Structure (by ref)"))
  (bind _assimple_character (cast `/Game/SimplePlatformerKit/Blueprints/Data/SimpleCharacter` OtherActor))
  (`/Game/SimplePlatformerKit/Blueprints/Data/SimpleCharacter.SendPlayerToLocation` _assimple_character (`/Game/SimplePlatformerKit/Blueprints/Data/SimpleCharacter.RespawnLocation` _assimple_character))
  (if (`self.ResetOnOverlap`)
    (set `self.ForcedStop` true)
    (`TimelineComponent.Stop` (`self.Movement`))
    (bind _output_get (set `self.Start` (`|GetArrayItem` (`self.Destinations`))))
    (`SceneComponent.K2_SetRelativeLocation` (`self.Pivot`) _output_get false false)
    (goto _label_2 :!via `Reset`)))

(fn `CheckKey`
  (params (KeyType :type "/Game/SimplePlatformerKit/Blueprints/Data/KeyType Enum" :default "NewEnumerator2"))
  (returns (Result :type Boolean))
  (return false))

(fn `UserConstructionScript`
  (`SceneComponent.SetRelativeScale3D` (`self.Pivot`) (`self.Size`))
  (`PrimitiveComponent.SetMaterial` (`self.Mesh`) 0 (`self.Material`))
  (bind _output_get (set `self.Start` (`|GetArrayItem` (`self.Destinations`) (`self.Index`))))
  (`SceneComponent.K2_SetRelativeLocation` (`self.Pivot`) _output_get false false))