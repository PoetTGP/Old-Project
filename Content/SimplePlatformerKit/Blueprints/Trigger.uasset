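; Trigger volume for the simple platformer kit that switches other objects on or off when a SimpleCharacter enters or leaves its Cube.
; Begin and end overlap events send SimpleActivateMessage and SimpleDeactivateMessage to separate target arrays for entry and exit.
; Separate entry and exit flags add DoOnce gates meant for one-time triggering.
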(event `self.Cube.OnComponentBeginOverlap`
  (params (OverlappedComponent :type "PrimitiveComponent Object Reference") (OtherActor :type "Actor Object Reference") (OtherComp :type "PrimitiveComponent Object Reference") (OtherBodyIndex :type Integer) (bFromSweep :type Boolean) (SweepResult :type "HitResult Structure (by ref)"))
  (cast `/Game/SimplePlatformerKit/Blueprints/Data/SimpleCharacter` OtherActor)
  (if (`self.TriggerEntryOnlyOnce`)
    (`/Engine/EditorBlueprintResources/StandardMacros.DoOnce` false
      (:`Completed`
        _)))
  (for _array_element (`self.ActivateOnEntry`)
    (message `/Game/SimplePlatformerKit/Blueprints/Data/SimpleBPI.SimpleActivate` _array_element))
  (for _array_element_2 (`self.DeactivateOnEntry`)
    (message `/Game/SimplePlatformerKit/Blueprints/Data/SimpleBPI.SimpleDeactivate` _array_element_2)))

(event `self.Cube.OnComponentEndOverlap`
  (params (OverlappedComponent :type "PrimitiveComponent Object Reference") (OtherActor :type "Actor Object Reference") (OtherComp :type "PrimitiveComponent Object Reference") (OtherBodyIndex :type Integer))
  (cast `/Game/SimplePlatformerKit/Blueprints/Data/SimpleCharacter` OtherActor)
  (if (`self.TriggerExitOnlyOnce`)
    (`/Engine/EditorBlueprintResources/StandardMacros.DoOnce` false
      (:`Completed`
        _)))
  (for _array_element (`self.ActivateOnExit`)
    (message `/Game/SimplePlatformerKit/Blueprints/Data/SimpleBPI.SimpleActivate` _array_element))
  (for _array_element_2 (`self.DeactivateOnExit`)
    (message `/Game/SimplePlatformerKit/Blueprints/Data/SimpleBPI.SimpleDeactivate` _array_element_2)))

(fn `UserConstructionScript`)