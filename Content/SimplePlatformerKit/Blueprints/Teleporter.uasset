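; Teleporter pad that sends an overlapping SimpleCharacter to just above its linked Destination actor.
; The box overlap passes the raised destination location to the character's SendPlayerToLocation.
; The construction script color-codes the link, applying Color to the pad's dynamic material, rising Niagara particles and Destination.
; It tracks PreviousDestination to reset that actor's material to black before coloring the current link.
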(event `self.Box.OnComponentBeginOverlap`
  (params (OverlappedComponent :type "PrimitiveComponent Object Reference") (OtherActor :type "Actor Object Reference") (OtherComp :type "PrimitiveComponent Object Reference") (OtherBodyIndex :type Integer) (bFromSweep :type Boolean) (SweepResult :type "HitResult Structure (by ref)"))
  (bind _assimple_character (cast `/Game/SimplePlatformerKit/Blueprints/Data/SimpleCharacter` OtherActor))
  (`/Engine/EditorBlueprintResources/StandardMacros.IsValid` (`self.Destination`)
    (:`Is Valid`
      (`/Game/SimplePlatformerKit/Blueprints/Data/SimpleCharacter.SendPlayerToLocation` _assimple_character (+ (`self.K2_GetActorLocation` (`self.Destination`)) (0.0 0.0 100.0))))))

(fn `UserConstructionScript`
  (bind _destination (`self.Destination`))
  (bind _destination_2 (`self.Destination`))
  (bind _previousdestination (`self.PreviousDestination`))
  (`/Engine/EditorBlueprintResources/StandardMacros.IsValid` _previousdestination
    (:`Is Valid`
      (`/Game/SimplePlatformerKit/Blueprints/Teleporter-Destination.AssignMaterial` _previousdestination (struct :`A` 1.0)))
    (:`Is Not Valid`
      _))
  (`/Engine/EditorBlueprintResources/StandardMacros.IsValid` _destination_2
    (:`Is Valid`
      (set `self.PreviousDestination` _destination_2)
      (bind _returnvalue (`PrimitiveComponent.CreateDynamicMaterialInstance` (`self.Pad`) 0 "/Game/SimplePlatformerKit/Materials/SimpleMaterial/AssetMaterials/MI_Teleporter.MI_Teleporter" "None"))
      (`MaterialInstanceDynamic.SetVectorParameterValue` _returnvalue "Color" (`self.Color`))
      (`NiagaraComponent.SetVariableLinearColor` (`self.NS_RisingParticles`) "TeleporterColor" (`self.Color`))
      (`/Engine/EditorBlueprintResources/StandardMacros.IsValid` _destination
        (:`Is Valid`
          (`/Game/SimplePlatformerKit/Blueprints/Teleporter-Destination.AssignMaterial` _destination (`self.Color`)))))
    (:`Is Not Valid`
      (set `self.PreviousDestination` null))))